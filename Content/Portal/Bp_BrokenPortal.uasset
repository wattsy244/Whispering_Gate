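; Broken portal actor that is replaced by a working Bp_Portal once enough parts have been built.
; BeginPlay sets the required part count, and each call to the Build event decrements it by one and prints the remainder.
; At zero the actor destroys itself and spawns Bp_Portal at its location, without carrying over rotation or scale.
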(event `self.ReceiveBeginPlay`
  (set `self.Total parts` 4.0))

(event `/Game/Portal/Bpi_Build.Build`
  (bind _output_get (set `self.CurrentParts` 1.0))
  (set `self.Total parts` (- (`self.Total parts`) _output_get))
  (`KismetSystemLibrary.PrintString` (`KismetStringLibrary.Conv_DoubleToString` (`self.Total parts`)))
  (if (== (`self.Total parts`) 0.0)
    (`self.K2_DestroyActor`)
    (`|SpawnActorFromClass` "/Game/Portal/Bp_Portal.Bp_Portal_C" (`KismetMathLibrary.Conv_VectorToTransform` (`self.K2_GetActorLocation`)) "Undefined" "MultiplyWithRoot" null null)
    (`KismetSystemLibrary.PrintString` "portal spawn")))

(fn `UserConstructionScript`)